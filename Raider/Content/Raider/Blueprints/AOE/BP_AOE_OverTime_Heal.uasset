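; Healing variant of an area-of-effect-over-time actor for Raider.
; On BeginPlay it binds Healing to the AOE overlap event, which sends a heal message of EffectAmount only when the overlapped actor is EffectTarget.
; A separate SetActorLocationToFloor event, not called in this graph, line-traces from a given target using its Z scaled by -1000 as the end and moves that target to the hit.
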(event Custom|SetActorLocationToFloor
  (params (HealTarget :type Actor%20Object%20Reference))
  (bind _returnvalue (Transformation|GetActorLocation HealTarget))
  (Utilities|IsValid HealTarget
    (:Is%20Valid
      ;[1 1 1] Perform a line trace from the actor to get the floor location
      (bind (_outhit _returnvalue_2) (Collision|LineTraceByChannel _returnvalue (* _returnvalue "1.000000,1.000000,-1000.000000") "TraceTypeQuery1" false (Utilities|Array|MakeArray HealTarget) "None"))
      (if _returnvalue_2
        (Transformation|SetActorLocation HealTarget (.Location (Collision|BreakHitResult _outhit)) false false)))))

(event Custom|Healing
  (params (Actor :type Actor%20Object%20Reference))
  (if (== Actor (Variables|Default|GetEffectTarget))
    (Class|MyCombatInterface|TakeHealing(Message) Actor (Variables|Default|GetEffectAmount))))

(event EventBeginPlay
  (|CallParentFunction)
  (EventDispatchers|BindEventtoOnAOEOverlapActor (delegate Custom|Healing)))

(fn ConstructionScript
  (|CallParentFunction))