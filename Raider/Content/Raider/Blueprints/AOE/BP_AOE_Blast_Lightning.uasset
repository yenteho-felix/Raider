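; Lightning blast AOE actor that telegraphs a strike on the floor beneath its attack target, then damages the actors it overlaps.
; On BeginPlay it line-traces from the target to snap itself to the floor, then spawns a target decal there.
; After a delay it triggers the inherited AOE and removes the decal.
; The AOE overlap event sends explosion-type hit damage, attributed to the instigator.
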(event Custom|SetActorLocationToFloor
  (bind _attacktarget (Variables|AOESettings|GetAttackTarget)
    (:then
      ;[1 1 1] Perform a line trace from the actor to get the floor location
      (bind (_outhit _returnvalue) (Collision|LineTraceByChannel (Transformation|GetActorLocation _attacktarget) (* (Transformation|GetActorLocation _attacktarget) "1.000000,1.000000,-1000.000000") "TraceTypeQuery1" false (Utilities|Array|MakeArray _attacktarget) "None"))
      (if _returnvalue
        (Transformation|SetActorLocation (.Location (Collision|BreakHitResult _outhit)) false false)))
    (:else)))

(event Custom|AOETelegraph
  ;[1 1 1] Spawn Decal
  (CallFunction|SetActorLocationtoFloor)
  (bind _returnvalue (Rendering|Decal|SpawnDecalatLocation "/Game/Assets/Textures/Decal/M_TargetDecal.M_TargetDecal" "20.000000,200.000000,200.000000" (Transformation|GetActorLocation) "-90.000000,0.000000,0.000000" 0.0))
  (Utilities|FlowControl|Delay (Variables|AOESettings|GetDelayBeforeStrike))
  (CallFunction|TriggerAOE)
  ;[1 1 1] Destory Decal
  (Utilities|IsValid _returnvalue
    (:Is%20Valid
      (Components|DestroyComponent _returnvalue))))

(event Custom|TakeDamage
  (params (Actor :type Actor%20Object%20Reference))
  (Class|MyCombatInterface|TakeDamage(Message) Actor (Variables|Default|GetInstigator) (Utilities|Struct|MakeSDamageInfo (Variables|Default|GetEffectAmount) "Explosion" "Hit" false false false)))

(event EventBeginPlay
  (|CallParentFunction)
  (CallFunction|AOETelegraph)
  (EventDispatchers|BindEventtoOnAOEOverlapActor (delegate Custom|TakeDamage)))

(fn ConstructionScript
  (|CallParentFunction))