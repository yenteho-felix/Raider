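; Actor component that gives its owner area-of-effect abilities: explosion, lightning strike, healing aura and fire aura.
; Each event spawns the matching AOE blast or over-time actor, passing the amount, any target and the owner pawn as instigator.
; The explosion spawns at the owner, ignores the instigator, and binds its overlap event to launch hit characters opposite their own facing direction.
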(event Custom|HealingAura
  (params (HealTarget :type Actor%20Object%20Reference) (HealAmount :type Float%20%28single-precision%29))
  (bind _returnvalue (Components|GetOwner))
  (bind (_aspawn _bsuccess) (Utilities|Casting|CastToPawn _returnvalue))
  (Game|SpawnActorfromClass "/Game/Raider/Blueprints/AOE/BP_AOE_OverTime_Heal.BP_AOE_OverTime_Heal_C" (Math|Transform|MakeTransform (Transformation|GetActorLocation HealTarget) "0, 0, 0" "1.000000,1.000000,1.000000") "Undefined" "MultiplyWithRoot" 0 HealTarget 1.0 5.0 HealTarget HealAmount false false true (select _bsuccess _aspawn 0)))

(event Custom|OnExplosion
  (params (Actor :type Actor%20Object%20Reference))
  ;[1 1 1] Push Character Backward
  (bind _ascharacter (Utilities|Casting|CastToCharacter Actor))
  (Character|LaunchCharacter _ascharacter (* (Math|Vector|NegateVector (Transformation|GetActorForwardVector Actor)) "500.000000,500.000000,500.000000") true false))

(event Custom|FireAura
  (params (AttackTarget :type Actor%20Object%20Reference) (AttackAmount :type Float%20%28single-precision%29))
  (bind _returnvalue (Components|GetOwner))
  (bind (_aspawn _bsuccess) (Utilities|Casting|CastToPawn _returnvalue))
  (Game|SpawnActorfromClass "/Game/Raider/Blueprints/AOE/BP_AOE_OverTime_Fire.BP_AOE_OverTime_Fire_C" (Math|Transform|MakeTransform (Transformation|GetActorLocation AttackTarget) "0, 0, 0" "1.000000,1.000000,1.000000") "Undefined" "MultiplyWithRoot" 0 1e+01 1.0 5.0 AttackTarget AttackAmount false false true (select _bsuccess _aspawn 0)))

(event Custom|Explosion
  (params (Damage%20Amount :type Float%20%28single-precision%29))
  (bind _returnvalue (Components|GetOwner))
  (bind (_aspawn _bsuccess) (Utilities|Casting|CastToPawn _returnvalue))
  (bind _returnvalue_2 (Game|SpawnActorfromClass "/Game/Raider/Blueprints/AOE/BP_AOE_Blast_Explosion.BP_AOE_Blast_Explosion_C" (Math|Transform|MakeTransform (Transformation|GetActorLocation _returnvalue) "0, 0, 0" "1.000000,1.000000,1.000000") "Undefined" "MultiplyWithRoot" 0 Damage%20Amount false true true (select _bsuccess _aspawn 0)))
  (EventDispatchers|AssignOnAOEOverlapActor _returnvalue_2 (delegate Custom|OnExplosion)))

(event Custom|LightningStrike
  (params (AttackTarget :type Actor%20Object%20Reference) (DelayBeforeStrike :type Float%20%28single-precision%29) (DamageAmount :type Float%20%28single-precision%29))
  (bind _returnvalue (Components|GetOwner))
  (bind (_aspawn _bsuccess) (Utilities|Casting|CastToPawn _returnvalue))
  (Game|SpawnActorfromClass "/Game/Raider/Blueprints/AOE/BP_AOE_Blast_Lightning.BP_AOE_Blast_Lightning_C" (Math|Transform|MakeTransform "0, 0, 0" "0, 0, 0" "1.000000,1.000000,1.000000") "Undefined" "MultiplyWithRoot" 0 DelayBeforeStrike AttackTarget DamageAmount false false false (select _bsuccess _aspawn 0)))