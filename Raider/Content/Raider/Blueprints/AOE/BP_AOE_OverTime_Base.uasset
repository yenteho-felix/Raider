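; Base Blueprint for an area-of-effect that lasts over time, extending a parent AOE class.
; On trigger it runs parent logic, plays effect and sound, then starts a looping interval timer for overlap pulses and a duration timer for destruction.
; The attached emitter is offset to the surface found by a downward trace from the effect target.
; Without a valid effect, the actor self-destructs after a short delay.
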(event Custom|PlayEffect
  (bind _effect (Variables|AOESettings|GetEffect)
    (:then
      (CallFunction|SetEmitterLocation)
      (Effects|SpawnEmitterAttached _effect (Variables|Transformation|GetRootComponent) "None" (Variables|Default|GetEmitterLocation)))
    (:else
      ;[1 1 1] Destroy Actor
      (Utilities|FlowControl|Delay 1.0)
      (Actor|DestroyActor))))

(event Custom|PlaySound
  (bind _sound (Variables|AOESettings|GetSound)
    (:then
      (Audio|PlaySoundatLocation _sound (Transformation|GetActorLocation) "0, 0, 0" 1.0 1.0 0.0 0 0 0 0))
    (:else)))

(event Custom|SetEmitterLocation
  (bind _effecttarget (Variables|AOESettings|GetEffectTarget)
    (:then
      (bind (_outhit _returnvalue) (Collision|LineTraceByChannel (Transformation|GetActorLocation _effecttarget) (* (Transformation|GetActorLocation _effecttarget) "1.000000,1.000000,-1000.000000") "TraceTypeQuery1" false (Utilities|Array|MakeArray _effecttarget) "None"))
      (if _returnvalue
        (Variables|Default|SetEmitterLocation (- (.Location (Collision|BreakHitResult _outhit)) (Transformation|GetActorLocation _effecttarget)))))
    (:else)))

(event EventTriggerAOE
  (|CallParentFunction)
  (CallFunction|PlayEffect)
  (CallFunction|PlaySound)
  (Utilities|FlowControl|Sequence
    (:then_0
      ;[1 1 1] Spawn AOE sphere to trigger actor overlap by interval
      (Utilities|Time|SetTimerbyEvent (EventDispatchers|CreateEvent :!event SpawnAOESphere) (Variables|AOESettings|GetEffectInterval) true))
    (:then_1
      ;[1 1 1] Destory this actor after duration
      (Utilities|Time|SetTimerbyEvent (EventDispatchers|CreateEvent :!event K2DestroyActor) (Variables|AOESettings|GetEffectDuration)))))

(fn ConstructionScript
  (|CallParentFunction))