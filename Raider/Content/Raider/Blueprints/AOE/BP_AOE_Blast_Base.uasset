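; Base Blueprint for a one-shot area-of-effect blast actor that adds visual and audio feedback when triggered.
; TriggerAOE runs the parent implementation, then attaches the effect emitter to the root component and plays the sound at the actor's location, each only if assigned.
; The actor destroys itself when the particle system finishes, or after a short delay when no effect is set.
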(event Custom|PlayEffect
  (bind _effect (Variables|AOESettings|GetEffect)
    (:then
      (bind _returnvalue (Effects|SpawnEmitterAttached _effect (Variables|Transformation|GetRootComponent) "None"))
      (EventDispatchers|BindEventtoOnSystemFinished _returnvalue (delegate Custom|SystemFinished)))
    (:else
      ;[1 1 1] Destory Actor
      (Utilities|FlowControl|Delay 1.0)
      (Actor|DestroyActor))))

(event Custom|PlaySound
  (bind _sound (Variables|AOESettings|GetSound)
    (:then
      (Audio|PlaySoundatLocation _sound (Transformation|GetActorLocation) "0, 0, 0" 1.0 1.0 0.0 0 0 0 0))
    (:else)))

(event Custom|SystemFinished
  (params (PSystem :type Particle%20System%20Component%20Object%20Reference))
  (Actor|DestroyActor))

(event EventTriggerAOE
  (|CallParentFunction)
  (CallFunction|PlayEffect)
  (CallFunction|PlaySound))

(fn ConstructionScript
  (|CallParentFunction))