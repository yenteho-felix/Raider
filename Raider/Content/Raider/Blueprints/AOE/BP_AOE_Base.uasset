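; BP_AOE_Base is a base area-of-effect actor that finds pawns within a radius of its location.
; It can trigger itself shortly after BeginPlay or through TriggerAOE, running a one-shot sphere overlap that can ignore the instigator.
; Each hit actor is broadcast through the OnAOEOverlapActor dispatcher, leaving the actual effect to whatever binds it.
; An optional debug mode draws the sphere and prints the overlapped actors.
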(event Custom|SpawnAOESphere
  (Utilities|FlowControl|Sequence
    (:then_0
      ;[1 1 1] Spawn an sphere that detects overlaps and fires the  AOEOverlapActor event
      (bind _outactors (Collision|SphereOverlapActors (Transformation|GetActorLocation) (Variables|AOESettings|GetEffectRadius) (Utilities|Array|MakeArray "ObjectTypeQuery3") 0 (select (Variables|AOESettings|GetbIgnoreInstigator) (Utilities|Array|MakeArray (Variables|Actor|GetInstigator)) 0)))
      (for _array_element _outactors
        (Default|CallOnAOEOverlapActor _array_element)
        ;[1 1 1] Debug Text
        (if (Variables|AOESettings|GetbDrawDebugSphere)
          (Development|PrintText (Utilities|Text|ToText(Object) _array_element)))))
    (:then_1
      ;[1 1 1] Debug Sphere
      (if (Variables|AOESettings|GetbDrawDebugSphere)
        (Rendering|Debug|DrawDebugSphere (Transformation|GetActorLocation) (Variables|AOESettings|GetEffectRadius) 12 "(R=1.000000,G=0.018175,B=0.000000,A=1.000000)" 2.0)))))

(event Custom|TriggerAOE
  (CallFunction|SpawnAOESphere))

(event EventBeginPlay
  (if (Variables|AOESettings|GetbTriggerOnBeginPlay)
    (Utilities|FlowControl|Delay 0.2)
    (CallFunction|TriggerAOE)))

(fn ConstructionScript)