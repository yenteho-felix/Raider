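; Enemy projectile attack component that fires White Magic and Dark Magic spells at a target actor.
; White Magic spawns three homing projectiles spaced evenly in a horizontal ring around the launch point, while Dark Magic fires one non-homing projectile.
; Launch points come from an enemy mesh socket, or the owner's transform if that socket is absent.
; Projectile hit events send damage through the combat interface, with White Magic explicitly blockable.
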(event Custom|DarkMagic
  (params (DamageAmout :type Float%20%28double-precision%29) (TargetActor :type Actor%20Object%20Reference))
  (bind _returnvalue (Components|GetOwner))
  (bind (_aspawn _bsuccess) (Utilities|Casting|CastToPawn _returnvalue))
  (bind _transform (CallFunction|GetTransformfromSocket))
  ;[1 1 1] Launch Projectile
  (bind _returnvalue_2 (Game|SpawnActorfromClass "/Game/Raider/Blueprints/Projectiles/BP_Projectile_DarkMagic.BP_Projectile_DarkMagic_C" _transform "Undefined" "MultiplyWithRoot" 0 8e+02 0.0 TargetActor false 2e+03 (select _bsuccess _aspawn 0)))
  ;[1 1 1] Call TakeDamage function from MyCombat Interface when projectile hits an actor
  (EventDispatchers|BindEventtoOnProjectileHit _returnvalue_2 (delegate Custom|CustomEvent_1)))

(event Custom|CustomEvent_1
  (params (Other%20Actor :type Actor%20Object%20Reference) (Hit :type Hit%20Result%20Structure))
  ;[1 1 1] Call TakeDamage function from MyCombat Interface when projectile hits an actor
  (Class|MyCombatInterface|TakeDamage(Message) Other%20Actor (stale Custom|DarkMagic _returnvalue_2) (Utilities|Struct|MakeSDamageInfo (stale Custom|DarkMagic DamageAmout) "Projectile" "Hit" false false false)))

(event Custom|WhiteMagic
  (params (DamageAmout :type Float%20%28double-precision%29) (TargetActor :type Actor%20Object%20Reference))
  (bind _returnvalue (Components|GetOwner))
  (bind (_aspawn _bsuccess) (Utilities|Casting|CastToPawn _returnvalue))
  (bind _transform (CallFunction|GetTransformfromSocket))
  ;[1 1 1] Launch Multiple Projects at Once
  (bind _spawntransforms (CallFunction|CalculateSpawnTransforms _transform 3 50))
  (for _array_element _spawntransforms
    ;[1 1 1] Launch Projectile
    (bind _returnvalue_2 (Game|SpawnActorfromClass "/Game/Raider/Blueprints/Projectiles/BP_Projectile_WhiteMagic.BP_Projectile_WhiteMagic_C" _array_element "Undefined" "MultiplyWithRoot" 0 6e+02 0.0 TargetActor true 2e+03 (select _bsuccess _aspawn 0)))
    ;[1 1 1] Call TakeDamage function from MyCombat Interface when projectile hits an actor
    (EventDispatchers|BindEventtoOnProjectileHit _returnvalue_2 (delegate Custom|DamageActor))))

(event Custom|DamageActor
  (params (Other%20Actor :type Actor%20Object%20Reference) (Hit :type Hit%20Result%20Structure))
  ;[1 1 1] Call TakeDamage function from MyCombat Interface when projectile hits an actor
  (Class|MyCombatInterface|TakeDamage(Message) Other%20Actor (stale Custom|WhiteMagic _returnvalue_2) (Utilities|Struct|MakeSDamageInfo (stale Custom|WhiteMagic DamageAmout) "Projectile" "Hit" false false true)))

(fn CalculateSpawnTransforms
  (params (StartTransform :type Transform) (Number :type Integer) (Radius :type Integer))
  (LocalVariables|SetAngle (/ 3.6e+02 Number))
  (for _index (range 0 (- Number 1))
    (Utilities|Array|Add (LocalVariables|GetTransformArray) (Math|Conversions|ToTransform(Vector) (+ (.location StartTransform) (* (Math|Vector|RotateVectorAroundAxis (Math|Vector|GetForwardVector (.rotation StartTransform)) (* _index (LocalVariables|GetAngle)) "0.000000,0.000000,1.000000") Radius)))))
  (return (LocalVariables|GetTransformArray)))

(fn GetTransformfromSocket
  (bind _returnvalue (Components|GetOwner))
  (bind _transformsocketname (Variables|ProjectileSettings|GetTransformSocketName))
  (bind _asbp_enemy_base (Utilities|Casting|CastToBP_EnemyBase _returnvalue))
  (Utilities|IsValid _asbp_enemy_base
    (:Is%20Valid
      (if (Transformation|DoesSocketExist (Variables|/Script/Engine.Character|GetMesh _asbp_enemy_base) _transformsocketname)
        (return (Transformation|GetSocketTransform (Variables|/Script/Engine.Character|GetMesh _asbp_enemy_base) _transformsocketname "RTS_World"))
        (else
          _)))
    (:Is%20Not%20Valid
      _))
  (return (Transformation|GetActorTransform _returnvalue)))