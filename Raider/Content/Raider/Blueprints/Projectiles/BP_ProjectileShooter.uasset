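; BP_ProjectileShooter is a placeable emitter that fires projectiles from its Arrow component on a looping timer.
; Each spawn receives speed and homing settings, with the player pawn passed as target.
; It binds each projectile's hit event and sends a fixed-damage TakeDamage message through the combat interface to the actor hit, naming the projectile as attacker.
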(event Custom|SpawnProjectile
  (bind _returnvalue (Game|SpawnActorfromClass (Variables|Settings|GetProjectileType) (Transformation|GetWorldTransform (Variables|Default|GetArrow)) "Undefined" "MultiplyWithRoot" self (Variables|Settings|GetSpeed) 0.0 (Game|Player|GetPlayerPawn 0) (Variables|Settings|GetbIsHoming) (Variables|Settings|GetHomingAcceleration) 0))
  ;[1 1 1] Call TakeDamage function from MyCombat Interface when projectile hits an actor
  (EventDispatchers|BindEventtoOnProjectileHit _returnvalue (delegate Custom|DamageActor)))

(event Custom|DamageActor
  (params (Other%20Actor :type Actor%20Object%20Reference) (Hit :type Hit%20Result%20Structure))
  ;[1 1 1] Call TakeDamage function from MyCombat Interface when projectile hits an actor
  (Class|MyCombatInterface|TakeDamage(Message) Other%20Actor (stale Custom|SpawnProjectile _returnvalue) (Utilities|Struct|MakeSDamageInfo 1e+01 "Projectile" "Hit" false false false)))

(event EventBeginPlay
  (Utilities|Time|SetTimerbyEvent (delegate Custom|SpawnProjectile) (Variables|Settings|GetFrequency) true))

(fn ConstructionScript)