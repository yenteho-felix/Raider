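; Base projectile actor that flies at a set speed and gravity, optionally aimed at or homing on a target.
; The construction script configures ProjectileMovement and enables homing on the target's root component when requested.
; BeginPlay ignores collision with the owner and points velocity at any valid target.
; On hit, it broadcasts OnProjectileHit, spawns the impact effect and sound, then destroys itself.
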(event OnComponentHit(BoxCollision)
  (params (HitComponent :type Primitive%20Component%20Object%20Reference) (OtherActor :type Actor%20Object%20Reference) (OtherComp :type Primitive%20Component%20Object%20Reference) (NormalImpulse :type Vector :default "0, 0, 0") (Hit :type Hit%20Result%20Structure%20%28by%20ref%29))
  (bind _location (Collision|BreakHitResult Hit))
  (Default|CallOnProjectileHit OtherActor Hit)
  (Effects|SpawnEmitteratLocation (Variables|Effects|GetHitEffect) _location)
  (Audio|PlaySoundatLocation (Variables|Effects|GetHitSound) _location "0, 0, 0" 1.0 1.0 0.0 0 0 0 0)
  (Actor|DestroyActor))

(event Custom|RotateToTarget
  ;[1 1 1] Set the projectile’s velocity by multiplying its direction to the target with the desired speed
  (Variables|/Script/Engine.MovementComponent|SetVelocity (Variables|Default|GetProjectileMovement) (* (Math|Vector|GetUnitDirection(Vector) (Transformation|GetActorLocation) (Transformation|GetActorLocation (Variables|ProjectileSettings|GetTarget))) (Variables|ProjectileSettings|GetSpeed))))

(event EventBeginPlay
  ;[1 1 1] Disable collision between the projectile and its owner
  (Collision|IgnoreActorwhenMoving (Variables|Default|GetBox%20Collision) (Components|GetOwner) true)
  (Variables|ProjectileSettings|GetTarget
    (:then
      (CallFunction|RotatetoTarget))
    (:else)))

(fn ConstructionScript
  (bind _projectilemovement (Variables|Default|GetProjectileMovement))
  ;[1 1 1] Speed & Gravity
  (Variables|/Script/Engine.ProjectileMovementComponent|SetInitialSpeed _projectilemovement (Variables|ProjectileSettings|GetSpeed))
  (Variables|/Script/Engine.ProjectileMovementComponent|SetMaxSpeed _projectilemovement (Variables|ProjectileSettings|GetSpeed))
  (Variables|/Script/Engine.ProjectileMovementComponent|SetProjectileGravityScale _projectilemovement (Variables|ProjectileSettings|GetGravity))
  ;[1 1 1] Homing Projectile
  (Variables|ProjectileSettings|GetTarget
    (:then
      (if (Variables|ProjectileSettings|GetbIsHoming)
        (Variables|/Script/Engine.ProjectileMovementComponent|SetbIsHomingProjectile _projectilemovement true)
        (Variables|/Script/Engine.ProjectileMovementComponent|SetHomingAccelerationMagnitude _projectilemovement (Variables|ProjectileSettings|GetHomingAcceleration))
        (Variables|/Script/Engine.ProjectileMovementComponent|SetHomingTargetComponent _projectilemovement (Variables|/Script/Engine.Actor|GetRootComponent (Variables|ProjectileSettings|GetTarget)))))
    (:else)))