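; BP_EnemyMage is a ranged enemy character that equips its weapon on BeginPlay and attacks its AI controller's current target.
; An attack montage notify fires a hitscan shot, using a multi-object Pawn line trace from the weapon actor to the target's location.
; The combat component applies Projectile-type damage with a Hit reaction to the first non-team member hit, without spawning a projectile.
; The trace's debug drawing is left enabled.
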(event EventBeginPlay
  (|CallParentFunction)
  (Class|MyCombatInterface|EquipWeapon self))

(event EventOnAttackMontageNotifyHandler
  (params (NotifyName :type Name :default "None"))
  (switch name NotifyName
    (:Fire
      ;[1 1 1] Fire Bullet
      (bind _asaic_enemy_base (Utilities|Casting|CastToAIC_EnemyBase (AI|GetAIController self)))
      (bind _attacktarget (Variables|/Script/Raider.NPCAIController|GetAttackTarget _asaic_enemy_base)
        (:then
          (bind _weaponactorobj (Variables|/Script/Raider.MyCombatComponent|GetWeaponActorObj (Variables|Default|GetCombatComponent))
            (:then
              (bind (_outhits _returnvalue) (Class|KismetSystemLibrary|LineTraceMultiforObjects (Transformation|GetActorLocation _weaponactorobj) (Transformation|GetActorLocation _attacktarget) (Utilities|Array|MakeArray "ObjectTypeQuery3") false (Utilities|Array|MakeArray (Components|GetOwner)) "ForDuration" true))
              (if _returnvalue
                (bind _returnvalue_2 (Class|MyCombatComponent|DamageFirstNoneTeamMembers (Variables|Default|GetCombatComponent) _outhits (Utilities|Struct|MakeSDamageInfo 1e+01 "Projectile" "Hit" false false false)))))
            (:else)))
        (:else)))))

(fn ConstructionScript
  (|CallParentFunction))