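; BP_PatrolRoute is a patrol path for NPCs, defined by the points of its PatrolRoute spline.
; It tracks a current point index and a direction, stepping the index on each increment and flipping direction at either end to ping-pong along the route.
; A getter returns the current spline point in world space, and a reset event restarts at the first point heading forward.
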(event Custom|IncrementPatrolRoute
  (bind _output_get (Variables|Default|SetPatrolIndex (+ (Variables|Default|GetPatrolIndex) (Variables|Default|GetDirection))))
  ;[1 1 1] End of PatroRoute, Move Backward
  (if (== _output_get (- (Spline|GetNumberOfSplinePoints (Variables|Default|GetPatrolRoute)) 1))
    (Variables|Default|SetDirection -1)
    (else
      ;[1 1 1] Start of PatroRoute, Move Forward
      (if (== (Variables|Default|GetPatrolIndex) 0)
        (Variables|Default|SetDirection 1)))))

(event Custom|ResetPatrolRoute
  (Variables|Default|SetPatrolIndex 0)
  (Variables|Default|SetDirection 1))

(fn ConstructionScript)

(fn GetSpinePointasWorldLocation
  (return (Spline|GetLocationatSplinePoint (Variables|Default|GetPatrolRoute) (Variables|Default|GetPatrolIndex) "World")))