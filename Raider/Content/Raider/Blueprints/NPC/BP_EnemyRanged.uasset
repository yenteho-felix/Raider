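; BP_EnemyRanged is a ranged enemy NPC that equips its weapon on BeginPlay and attacks through its CombatComponent's attack montage.
; A montage notify fires a hitscan shot from the weapon actor toward the AIC_EnemyBase controller's AttackTarget, using a debug-drawn Visibility trace.
; Fixed projectile-type damage applies only when the trace hits nothing, so it acts as a line-of-sight check.
; Montage completion or interruption notifies the CombatComponent.
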(event EventBeginPlay
  (|CallParentFunction)
  (Class|MyCombatInterface|EquipWeapon self))

(event EventAttack
  (bind _combatcomponent (Variables|Default|GetCombatComponent))
  (bind _attackmontage (Variables|/Script/Raider.MyCombatComponent|GetAttackMontage _combatcomponent))
  ;[1 1 1] Play AttackMontage
  (Utilities|IsValid _attackmontage
    (:Is%20Valid
      (bind _notifyname (Animation|Montage|PlayMontage (Variables|Character|GetMesh) _attackmontage)
        (:OnCompleted
          (Class|MyCombatComponent|OnAttackMontageEnded (Variables|Default|GetCombatComponent) 0 false :!label _label))
        (:OnInterrupted
          (goto _label))
        (:OnNotifyBegin
          ;[1 1 1] Fire Bullet
          (switch name _notifyname
            (:Fire
              (bind _asaic_enemy_base (Utilities|Casting|CastToAIC_EnemyBase (AI|GetAIController self)))
              (bind _attacktarget (Variables|/Script/Raider.NPCAIController|GetAttackTarget _asaic_enemy_base)
                (:then
                  (bind _weaponactorobj (Variables|/Script/Raider.MyCombatComponent|GetWeaponActorObj (Variables|Default|GetCombatComponent))
                    (:then
                      (bind _returnvalue (Collision|LineTraceByChannel (Transformation|GetActorLocation _weaponactorobj) (Transformation|GetActorLocation _attacktarget) "TraceTypeQuery1" false 0 "ForDuration"))
                      (if (not _returnvalue)
                        (Class|MyCombatInterface|TakeDamage(Message) _attacktarget (Utilities|Struct|MakeSDamageInfo 1e+01 "Projectile" "Hit" false false false))))
                    (:else)))
                (:else)))))))))

(fn ConstructionScript
  (|CallParentFunction))