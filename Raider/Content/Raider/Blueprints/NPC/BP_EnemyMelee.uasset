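; Melee enemy NPC for the Raider game that carries a weapon and performs a montage-driven attack.
; On BeginPlay it spawns the weapon actor, snaps it to the right-hand sword socket on the mesh, stores the attach result as IsWeaponEquipped and fires OnEquipWeaponEnd.
; Attack plays the steel melee montage and fires OnAttackEnd on either completion or interruption, so listeners are notified in both cases.
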(event EventBeginPlay
  (Class|NPCCombatInterface|EquipWeapon self))

(event EventEquipWeapon
  (bind _returnvalue (Game|SpawnActorfromClass (Variables|Default|GetWeaponActor) (Transformation|GetActorTransform) "Undefined" "MultiplyWithRoot" 0 0))
  (bind _returnvalue_2 (Transformation|AttachComponentToComponent _returnvalue (Variables|Character|GetMesh) "hand_r_sword_socket" "SnapToTarget" "SnapToTarget" "SnapToTarget" true))
  (Variables|Default|SetIsWeaponEquipped _returnvalue_2)
  (Class|NPCCharacterBase|TriggeronEquipWeaponEnd))

(event EventAttack
  (Animation|Montage|PlayMontage (Variables|Character|GetMesh) "/Game/Characters/Steel/MM_Steel_Attack_Melee_A_Montage.MM_Steel_Attack_Melee_A_Montage"
    (:OnCompleted
      _)
    (:OnInterrupted
      _))
  (Class|NPCCharacterBase|TriggeronAttackEnd))

(fn ConstructionScript)