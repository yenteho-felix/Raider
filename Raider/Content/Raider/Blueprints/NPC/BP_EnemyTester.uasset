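; BP_EnemyTester is an NPC enemy for testing attacks from the BPCAttacks component against the player.
; On BeginPlay it stores the player character as its target and, if AttackPlayer is set, starts a looping timer that sends an Attack message with that target.
; Its Attack event calls a delayed, damaging LightningStrike on the component.
; A HealingAura call is present but left unconnected.
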(event Custom|DoAttack
  (Class|MyCombatInterface|Attack(Message) self (stale EventBeginPlay _output_get)))

(event EventBeginPlay
  (|CallParentFunction)
  (bind _output_get (Variables|Default|SetTarget (Game|GetPlayerCharacter 0)))
  (if (Variables|Default|GetbAttackPlayer)
    (Utilities|Time|SetTimerbyEvent (delegate Custom|DoAttack) 3.0 true)))

(event EventAttack
  (params (AttackTarget :type Actor%20Object%20Reference))
  (Default|LightningStrike (Variables|Default|GetBPC_Attacks) AttackTarget 2.0 1e+01))

(fn ConstructionScript
  (|CallParentFunction))