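; Player character Blueprint whose event graph holds only debug hotkeys for testing enemy AI states and perception.
; Key 1 flip-flops a melee enemy's AIC_EnemyBase controller between attacking the player and passive.
; Key 2 emits an AI-audible noise with explosion effects at the player.
; Key 3 reports a damage sense event and separately applies damage to a ranged enemy, with sound and particle feedback.
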(event Input|KeyboardEvents|1
  (params (Key :type Key%20Structure :default "None"))
  ;[1 1 1] Debug - Press 1 to change enemy state
  (:Pressed
    (bind _returnvalue (Actor|GetActorOfClass "/Game/Raider/Blueprints/NPC/BP_EnemyMelee.BP_EnemyMelee_C"))
    (bind _asaic_enemy_base (Utilities|Casting|CastToAIC_EnemyBase (AI|GetAIController _returnvalue)))
    (Utilities|FlowControl|FlipFlop
      (:A
        (Class|NPCAIController|SetStateasAttacking _asaic_enemy_base (Game|Player|GetPlayerPawn 0)))
      (:B
        (Class|NPCAIController|SetStateasPassive _asaic_enemy_base)))))

(event Input|KeyboardEvents|2
  (params (Key :type Key%20Structure :default "None"))
  (bind _returnvalue (Transformation|GetActorLocation))
  ;[1 1 1] Debug - Press 2 to make noise so AI can react to it
  (:Pressed
    (Class|Actor|MakeNoise 1.0 self _returnvalue 0.0 "None") ; Make Noise Itself allows AI to detect noise already
    (Effects|SpawnEmitteratLocation "/Game/Assets/StarterContent/Particles/P_Explosion.P_Explosion" _returnvalue)
    (Audio|PlaySoundatLocation "/Game/Assets/StarterContent/Audio/Explosion01.Explosion01" _returnvalue "0, 0, 0" 1.0 1.0 0.0 0 0 0 0)))

(event Input|KeyboardEvents|3
  (params (Key :type Key%20Structure :default "None"))
  (bind _returnvalue (Transformation|GetActorLocation))
  ;[1 1 1] Debug - Press 3 to make damage to AI
  (:Pressed
    (bind _returnvalue_2 (Actor|GetActorOfClass "/Game/Raider/Blueprints/NPC/BP_EnemyRanged.BP_EnemyRanged_C"))
    (Class|AISenseDamage|ReportDamageEvent _returnvalue_2 self 1e+01 _returnvalue _returnvalue "None")
    (Audio|PlaySoundatLocation "/Game/Raider/Audio/Sounds/Weapons/Rifle/Weapons_Rifle_Noise-Exterior-Distant_01.Weapons_Rifle_Noise-Exterior-Distant_01" _returnvalue "0, 0, 0" 1.0 1.0 0.0 0 0 0 0)
    (Effects|SpawnEmitteratLocation "/Game/Assets/StarterContent/Particles/P_Explosion.P_Explosion" (Transformation|GetActorLocation _returnvalue_2))
    (Game|Damage|ApplyDamage _returnvalue_2 2e+01 0 self)))

(fn ConstructionScript)